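; Player actor that rides a track actor's spline like a coaster car, looping back to the start past the track's end.
; Each Tick, helper functions for pitch-based gravity, added velocity and braking adjust CurrentSpeed, which is held at MinSpeed or above.
; While Climbing, those are skipped and speed interpolates at a constant rate toward a climbing speed.
; Speed advances Distance along the spline, which sets actor location and rotation.
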(event EventBeginPlay
  (Utilities|FlowControl|Sequence
    (:then_0
      (Variables|Default|SetEachTrackLEnght (Spline|GetSplineLength (Variables|/Game/MyContent/TestPline/Track_Bp.Track_Bp_C|GetSpline (Variables|Default|GetTrack_Actor)))))))

(event EventTick
  (params (DeltaSeconds :type Float%20%28single-precision%29))
  (bind _minspeed (Variables|Default|GetMinSpeed))
  (Utilities|FlowControl|Sequence
    (:then_0
      (if (Variables|Default|GetClimbing)
        _
        (else
          (bind _output_get (Variables|Default|SetCurrentSpeed (+ (Variables|Default|GetCurrentSpeed) (|Calculate_Gravity))))
          (Variables|Default|SetCurrentSpeed (+ _output_get (|Adding_Velocity) (|Calculate_brake)))
          (Variables|Default|SetAddingVelocityPendingOnce false)))
      (Variables|Default|SetDistance (|Calulate_Distance))
      (|PlayerLocationandRotation))
    (:then_1
      (Utilities|FlowControl|Sequence
        (:then_0
          (if (> (Variables|Default|GetAddingVelocity) 0.0)
            (Variables|Default|SetAddingVelocityDuration (- (Variables|Default|GetAddingVelocity) (Utilities|Time|GetWorldDeltaSeconds)))
            (elif (not (Variables|Default|GetAddingVelocityPendingOnce))
              (Variables|Default|SetAddingVelocity 0.0)
              (Variables|Default|SetAddingVelocityDuration 0.0))))
        (:then_1
          (if (and (<= (Variables|Default|GetCurrentSpeed) (Variables|Default|GetMinSpeed)) (> (Variables|Default|GetBrake) 0.0))
            (Variables|Default|SetBrake 0.0)))
        (:then_2
          (if (Variables|Default|GetClimbing)
            (if (!= (Variables|Default|GetCurrentSpeed) (Variables|Default|GetClimingSpeed))
              (Variables|Default|SetCurrentSpeed (Math|Interpolation|FInterptoConstant (Variables|Default|GetCurrentSpeed) (Variables|Default|GetClimingSpeed) (Utilities|Time|GetWorldDeltaSeconds) (Variables|Default|GetClimbingInterpolationSpeed))))
            (elif (< (Variables|Default|GetCurrentSpeed) _minspeed)
              (Variables|Default|SetCurrentSpeed _minspeed))))))
    (:then_2
      (Variables|Default|SettxtSpeed (Utilities|Text|ToText(Float) (Variables|Default|GetCurrentSpeed) "HalfToEven")))))

(fn ConstructionScript)

(fn GetPitch
  (return (/ (- (Math|Float|Absolute(Float) (.Pitch (Math|Rotator|BreakRotator (Math|Rotator|Delta(Rotator) (Spline|GetRotationatDistanceAlongSpline (Variables|/Game/MyContent/TestPline/Track_Bp.Track_Bp_C|GetSpline (Variables|Default|GetTrack_Actor)) (Variables|Default|GetDistance) "Local") "0, 0, 0")))) 9e+01) 9e+01)))